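; BP_FightManager sets up and starts a boxing match between two boxers, also serving as the player's view target.
; Construction positions the boxers; BeginPlay creates the HUD with both boxers, binds its options-confirmed event and switches to UI-only input with a visible cursor.
; The fight-start order plays background music and fidget moves, then starts the fight after a short delay.
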(event `self.ReceiveBeginPlay`
  (bind _returnvalue (`GameplayStatics.GetPlayerController` 0))
  (bind _returnvalue_2 (`|CreateWidget` "/Game/_PA/UserInterface/W_HUD.W_HUD_C" null (`self.FirstBoxer`) (`self.SecondBoxer`)))
  (add `/Game/_PA/UserInterface/W_HUD.OptionsConfirmed` _returnvalue_2 (`|CreateDelegate` :!event `OrderStartTheFight`))
  (`UserWidget.AddToViewport` _returnvalue_2 0)
  (`PlayerController.SetViewTargetWithBlend` (`GameplayStatics.GetPlayerController` 0) self 0.0 "VTBlend_Linear" 0.0 false)
  (`WidgetBlueprintLibrary.SetInputMode_UIOnlyEx` _returnvalue null)
  (set `PlayerController.bShowMouseCursor` true _returnvalue))

(event `self.OrderStartTheFight`
  (`GameplayStatics.PlaySound2D` "/Game/_PA/Audio/Music/Metasounds/MS_BackgroundMusic.MS_BackgroundMusic" 1.0 1.0 0.0 null null)
  (`self.PerformBoxersFidgetMoves`)
  (`KismetSystemLibrary.Delay` 2.4)
  (`self.StartTheFight`))

(fn `UserConstructionScript`
  (`self.PositionBoxers`))